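; Procedural level generator that fills a 3D grid with connection-matched tile actors, using a Wave Function Collapse style algorithm.
; Each slot starts with a weighted copy of TileSet, and generation begins at a fixed or random slot.
; Tick propagates constraints by purging incompatible neighbor options, then spawns a random candidate in the open connected slot with fewest options.
; Debug options lay out the tileset in a row instead or draw tile bounds.
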(event `self.ReceiveBeginPlay`
  (if (`self.Debug Tileset`)
    (for (_array_element _array_index) (`self.Tile Set`)
      (`|SpawnActorFromClass` _array_element (`KismetMathLibrary.MakeTransform` (`KismetMathLibrary.MakeVector` (* (* _array_index (`self.Tile Spacing`)) 2.0))) "Undefined" "MultiplyWithRoot" null null))
    (else
      (`KismetSystemLibrary.DrawDebugBox` (0.0 0.0 0.0) (* (`KismetMathLibrary.Conv_IntVectorToVector` (`self.Level Size`)) (/ (`self.Tile Spacing`) 2.0)) (struct :`B` 1.0 :`A` 1.0) (struct) 300.0 5.0)
      (`self.Generate Grid`)
      (`self.Spawn Tile` (`self.Current Slot`))
      (set `self.Purge Slots` true))))

(event `Try Spawn Next Tile Again`
  (`KismetSystemLibrary.DelayUntilNextTick`)
  (`KismetSystemLibrary.PrintString` "Try Spawning Next Tile Again" true true (struct :`R` 1.0 :`B` 0.016666 :`A` 1.0))
  (`self.Spawn Next Tile`))

(event `self.ReceiveTick`
  (params (DeltaSeconds :type "Float (single-precision)"))
  (bind _slots_to_purge (`self.Slots To Purge`))
  (bind _purge_slots (`self.Purge Slots`))
  (if (not (`self.Generation Complete`))
    (if _purge_slots
      (for _ (range (+ (`self.Purge Cycles Per Tick`) 1))
        (if (> (`KismetArrayLibrary.Array_Length` _slots_to_purge) 0)
          (`self.Purge Slot` (`|GetArrayItem` _slots_to_purge))
          (`KismetArrayLibrary.Array_Remove` _slots_to_purge)
          (else
            (set `self.Purge Slots` false)
            (break))))
      (if (not _purge_slots)
        (`self.Spawn Next Tile`)))))

(fn `Add Int Vector`
  (params (`Int Vector A In` :type "IntVector Structure") (`Int Vector B In` :type "IntVector Structure (by ref)"))
  (returns (`Int Vector Out` :type "IntVector Structure"))
  (return (`KismetMathLibrary.FTruncVector` (+ `Int Vector A In` `Int Vector B In`))))

(fn `Create Connections Array`
  (params (`Slot Index In` :type "IntVector Structure (by ref)"))
  (returns (`Connections Array Out` :type "Array of /Game/Blueprints/Structures/Connections/TileConnectionsArray Structure"))
  (locals (`Temp Source Connection Array` :type "Array of /Game/Blueprints/Structures/Connections/TileConnectionsArray Structure"))
  (bind _slot_out (`self.Get Slot` `Slot Index In`))
  (for _array_element (break `/Game/Blueprints/Structures/LevelGrid/MyTileSlot` _slot_out)
    (bind _array (`self.Get Tile Connections As Array` _array_element))
    (for (_array_element_2 _array_index) _array
      (bind _output_connections (break `/Game/Blueprints/Structures/Connections/TileConnectionsArray` (`|GetArrayItem` (`local.Temp Source Connection Array`) _array_index)))
      (`KismetArrayLibrary.Array_AddUnique` _output_connections _array_element_2)))
  (return (`local.Temp Source Connection Array`)))

(fn `Create Grid`
  (params (`Grid Size In` :type "IntVector Structure (by ref)") (`My Tiles In` :type "Array of /Game/Blueprints/MyTile Class Reference"))
  (returns (`Grid Out` :type "/Game/Blueprints/Structures/LevelGrid/MyTileGridX Structure"))
  (bind (_x _y _z) (break `IntVector` `Grid Size In`))
  (bind _mytilegridx (make `/Game/Blueprints/Structures/LevelGrid/MyTileGridX` _))
  (bind _mytilegridy (make `/Game/Blueprints/Structures/LevelGrid/MyTileGridY` _))
  (bind _mytilegridz (make `/Game/Blueprints/Structures/LevelGrid/MyTileGridZ` _))
  (bind _yaxis (break `/Game/Blueprints/Structures/LevelGrid/MyTileGridX` _mytilegridx))
  (bind _zaxis (break `/Game/Blueprints/Structures/LevelGrid/MyTileGridY` _mytilegridy))
  (bind _tileslots (break `/Game/Blueprints/Structures/LevelGrid/MyTileGridZ` _mytilegridz))
  (`KismetArrayLibrary.Array_Resize` _yaxis _x)
  (`KismetArrayLibrary.Array_Resize` _zaxis _y)
  (`KismetArrayLibrary.Array_Resize` _tileslots _z)
  (for (_ _array_index) _tileslots
    (`KismetArrayLibrary.Array_Set` _tileslots _array_index (make `/Game/Blueprints/Structures/LevelGrid/MyTileSlot` `My Tiles In`)))
  (for (_ _array_index_2) _zaxis
    (`KismetArrayLibrary.Array_Set` _zaxis _array_index_2 _mytilegridz))
  (for (_ _array_index_3) _yaxis
    (`KismetArrayLibrary.Array_Set` _yaxis _array_index_3 _mytilegridy))
  (return _mytilegridx))

(fn `Generate Grid`
  (locals (`Temp My Tiles` :type "Array of /Game/Blueprints/MyTile Class Reference"))
  (bind _starting_pos (`self.Starting Pos`))
  (bind (_level_size_x _level_size_y _level_size_z) (break `IntVector` (`self.Level Size`)))
  (bind _starting_tile (`self.Starting Tile`))
  (bind _int_vector_out (`self.Add Int Vector` _starting_pos (make `IntVector` -1 -1 -1)))
  (bind _int_vector_out_2 (`self.Add Int Vector` (`self.Starting Range Max`) (make `IntVector` -1 -1 -1)))
  (bind _int_vector_out_3 (`self.Add Int Vector` (`self.Starting Range Min`) (make `IntVector` -1 -1 -1)))
  (bind (_x _y _z) (break `IntVector` _int_vector_out_2))
  (bind (_x_2 _y_2 _z_2) (break `IntVector` _int_vector_out_3))
  (for _array_element (`self.Tile Set`)
    (for _ (range 1 (+ (defaults `Object` _array_element) 1))
      (`KismetArrayLibrary.Array_Add` (`local.Temp My Tiles`) _array_element)))
  (set `self.Grid` (`self.Create Grid` (`self.Level Size`) (`local.Temp My Tiles`)))
  (switch `/Game/Blueprints/GenerationParameters` (`self.GenerationStartingParameter`)
    (:`NewEnumerator0`
      (if (`self.Validate Slot` _int_vector_out)
        (set `self.Current Slot` _int_vector_out)
        (`KismetSystemLibrary.PrintString` (`KismetStringLibrary.Conv_IntVectorToString` _starting_pos) true true (struct :`G` 0.66 :`B` 1.0 :`A` 1.0) 60.0)
        (if (`KismetSystemLibrary.IsValidClass` _starting_tile) :!label _label
          (`self.Set Slot` (`self.Current Slot`) (make `/Game/Blueprints/Structures/LevelGrid/MyTileSlot` (`|MakeArray` _starting_tile))))
        (return)
        (else
          (`KismetSystemLibrary.PrintString` "Starting Pos Out Of Range" true true (struct :`R` 1.0 :`G` 0.016667 :`A` 1.0) 60.0))))
    (:`NewEnumerator1`
      (if (and (`self.Validate Slot` _int_vector_out_3) (`self.Validate Slot` _int_vector_out_2))
        (bind _output_get (set `self.Current Slot` (make `IntVector` (`KismetMathLibrary.RandomIntegerInRange` _x_2 _x) (`KismetMathLibrary.RandomIntegerInRange` _y_2 _y) (`KismetMathLibrary.RandomIntegerInRange` _z_2 _z))))
        (`KismetSystemLibrary.PrintString` (`KismetStringLibrary.Conv_IntVectorToString` (`self.Add Int Vector` _output_get (make `IntVector` 1 1 1))) true true (struct :`G` 0.66 :`B` 1.0 :`A` 1.0) 60.0)
        (goto _label)
        (else
          (`KismetSystemLibrary.PrintString` "Random Starting Pos Out Of Range" true true (struct :`R` 1.0 :`G` 0.016667 :`A` 1.0) 60.0))))
    (:`NewEnumerator2`
      (bind _output_get_2 (set `self.Current Slot` (make `IntVector` (`KismetMathLibrary.RandomIntegerInRange` 0 (- _level_size_x 1)) (`KismetMathLibrary.RandomIntegerInRange` 0 (- _level_size_y 1)) (`KismetMathLibrary.RandomIntegerInRange` 0 (- _level_size_z 1)))))
      (`KismetSystemLibrary.PrintString` (`KismetStringLibrary.Conv_IntVectorToString` _output_get_2) true true (struct :`G` 0.66 :`B` 1.0 :`A` 1.0) 60.0)
      (goto _label))))

(fn `Get Directional Vectors`
  (returns (Array :type "Array of IntVector Structure"))
  (return (`|MakeArray` (`KismetMathLibrary.FTruncVector` (`KismetMathLibrary.Vector_Forward`)) (`KismetMathLibrary.FTruncVector` (`KismetMathLibrary.Vector_Backward`)) (`KismetMathLibrary.FTruncVector` (`KismetMathLibrary.Vector_Right`)) (`KismetMathLibrary.FTruncVector` (`KismetMathLibrary.Vector_Left`)) (`KismetMathLibrary.FTruncVector` (`KismetMathLibrary.Vector_Up`)) (`KismetMathLibrary.FTruncVector` (`KismetMathLibrary.Vector_Down`)))))

(fn `Get Grid Size`
  (returns (`Grid Size Out` :type "IntVector Structure"))
  (bind _yaxis (break `/Game/Blueprints/Structures/LevelGrid/MyTileGridX` (`self.Grid`)))
  (bind _zaxis (break `/Game/Blueprints/Structures/LevelGrid/MyTileGridY` (`|GetArrayItem` _yaxis)))
  (return (make `IntVector` (`KismetArrayLibrary.Array_Length` _yaxis) (`KismetArrayLibrary.Array_Length` _zaxis) (`KismetArrayLibrary.Array_Length` (`.TileSlots_4_070D6DA14DE285DA696B848F45A7A9A6` (break `/Game/Blueprints/Structures/LevelGrid/MyTileGridZ` (`|GetArrayItem` _zaxis)))))))

(fn `Get Slot`
  (params (`Slot Index In` :type "IntVector Structure (by ref)"))
  (returns (`Slot Out` :type "/Game/Blueprints/Structures/LevelGrid/MyTileSlot Structure (by ref)"))
  (bind (_x _y _z) (break `IntVector` `Slot Index In`))
  (if (`self.Validate Slot` `Slot Index In`)
    (return (`|GetArrayItem` (`.TileSlots_4_070D6DA14DE285DA696B848F45A7A9A6` (break `/Game/Blueprints/Structures/LevelGrid/MyTileGridZ` (`|GetArrayItem` (`.ZAxis_3_2D884935497BCE97B635888E43E3AA98` (break `/Game/Blueprints/Structures/LevelGrid/MyTileGridY` (`|GetArrayItem` (`.YAxis_3_B19D8BF7491D421C533931BC366B0A92` (break `/Game/Blueprints/Structures/LevelGrid/MyTileGridX` (`self.Grid`))) _x))) _y))) _z))))

(fn `Get Tile Connections`
  (params (`My Tile In` :type "/Game/Blueprints/MyTile Class Reference"))
  (returns (`Forward (+X)` :type "/Game/Blueprints/ConnectionKeys Enum") (`Backward (-X)` :type "/Game/Blueprints/ConnectionKeys Enum") (`Right (+Y)` :type "/Game/Blueprints/ConnectionKeys Enum") (`Left (-Y)` :type "/Game/Blueprints/ConnectionKeys Enum") (`Up (+Z)` :type "/Game/Blueprints/ConnectionKeys Enum") (`Down (-Z)` :type "/Game/Blueprints/ConnectionKeys Enum"))
  (bind (_forward_x _backward_x _right_y _left_y _up_z _down_z) (break `/Game/Blueprints/Structures/Connections/TileConnections` (`.Tile Connections` (defaults `Object` `My Tile In`))))
  (return _forward_x _backward_x _right_y _left_y _up_z _down_z))

(fn `Get Tile Connections As Array`
  (params (`My Tile In` :type "/Game/Blueprints/MyTile Class Reference"))
  (returns (Array :type "Array of /Game/Blueprints/ConnectionKeys Enum"))
  (bind (_forward_x _backward_x _right_y _left_y _up_z _down_z) (break `/Game/Blueprints/Structures/Connections/TileConnections` (`.Tile Connections` (defaults `Object` `My Tile In`))))
  (if (`KismetSystemLibrary.IsValidClass` `My Tile In`)
    (return (`|MakeArray` _forward_x _backward_x _right_y _left_y _up_z _down_z))))

(fn `Get Tile Connections As Reversed Array`
  (params (`My Tile In` :type "/Game/Blueprints/MyTile Class Reference"))
  (returns (Array :type "Array of /Game/Blueprints/ConnectionKeys Enum"))
  (bind (_forward_x _backward_x _right_y _left_y _up_z _down_z) (break `/Game/Blueprints/Structures/Connections/TileConnections` (`.Tile Connections` (defaults `Object` `My Tile In`))))
  (return (`|MakeArray` _backward_x _forward_x _left_y _right_y _down_z _up_z)))

(fn `Get Tile Pos`
  (params (`Slot Index In` :type "IntVector Structure (by ref)"))
  (returns (`Tile Position Out` :type "Vector Structure"))
  (bind _tile_spacing (`self.Tile Spacing`))
  (return (`KismetMathLibrary.MakeVector` (* (- (.x (`KismetMathLibrary.Conv_IntVectorToVector` `Slot Index In`)) (/ (- (.x (`KismetMathLibrary.Conv_IntVectorToVector` (`self.Get Grid Size`))) 1.0) 2.0)) _tile_spacing) (* (- (.y (`KismetMathLibrary.Conv_IntVectorToVector` `Slot Index In`)) (/ (- (.y (`KismetMathLibrary.Conv_IntVectorToVector` (`self.Get Grid Size`))) 1.0) 2.0)) _tile_spacing) (* (- (.z (`KismetMathLibrary.Conv_IntVectorToVector` `Slot Index In`)) (/ (- (.z (`KismetMathLibrary.Conv_IntVectorToVector` (`self.Get Grid Size`))) 1.0) 2.0)) _tile_spacing))))

(fn `Purge Slot`
  (params (`Slot In` :type "IntVector Structure"))
  (returns (`Next Slots Out` :type "Array of IntVector Structure"))
  (locals (`Source Slot` :type "IntVector Structure") (`Source Slot Connections` :type "Array of /Game/Blueprints/Structures/Connections/TileConnectionsArray Structure") (`Temp Neighbor Slot` :type "IntVector Structure") (`Temp Slot Updated` :type Boolean) (`Temp Tiles` :type "Array of /Game/Blueprints/MyTile Class Reference") (`Next Slots` :type "Array of IntVector Structure"))
  (bind _temp_neighbor_slot (`local.Temp Neighbor Slot`))
  (if (`self.Validate Slot` `Slot In`)
    (bind _output_get (set `local.Source Slot` `Slot In`))
    (bind _connections_array_out (`self.Create Connections Array` _output_get))
    (set `local.Source Slot Connections` _connections_array_out)
    (for (_array_element _array_index) (`self.Get Directional Vectors`)
      (`KismetArrayLibrary.Array_Clear` (`local.Temp Tiles`))
      (set `local.Temp Slot Updated` false)
      (bind _int_vector_out (`self.Add Int Vector` _array_element (`local.Source Slot`)))
      (set `local.Temp Neighbor Slot` _int_vector_out)
      (bind _slot_out (`self.Get Slot` _int_vector_out))
      (if (`self.Validate Slot` _int_vector_out)
        (if (> (`KismetArrayLibrary.Array_Length` (break `/Game/Blueprints/Structures/LevelGrid/MyTileSlot` _slot_out)) 1)
          (for _array_element_2 (break `/Game/Blueprints/Structures/LevelGrid/MyTileSlot` _slot_out)
            (bind _output_connections (break `/Game/Blueprints/Structures/Connections/TileConnectionsArray` (`|GetArrayItem` (`local.Source Slot Connections`) _array_index)))
            (if (`KismetArrayLibrary.Array_Contains` _output_connections (`|GetArrayItem` (`self.Get Tile Connections As Reversed Array` _array_element_2) _array_index))
              (`KismetArrayLibrary.Array_AddUnique` (`local.Temp Tiles`) _array_element_2)
              (else
                (set `local.Temp Slot Updated` true))))
          (if (`local.Temp Slot Updated`)
            (`self.Set Slot` _temp_neighbor_slot (make `/Game/Blueprints/Structures/LevelGrid/MyTileSlot` (`local.Temp Tiles`)))
            (`KismetArrayLibrary.Array_Add` (`self.Slots To Purge`) _temp_neighbor_slot))
          (else
            (`self.Spawn Neighbor Tile` _int_vector_out _array_index (`.TileSpawned_9_E5F479944C63E28DBE795DA58B6154F7` (break `/Game/Blueprints/Structures/LevelGrid/MyTileSlot` _slot_out)))))))
    (return (`local.Next Slots`))))

(fn `Set Slot`
  (params (`Slot Index In` :type "IntVector Structure (by ref)") (`New Slot In` :type "/Game/Blueprints/Structures/LevelGrid/MyTileSlot Structure (by ref)"))
  (returns (`Slot Out` :type "/Game/Blueprints/Structures/LevelGrid/MyTileSlot Structure (by ref)"))
  (bind (_x _y _z) (break `IntVector` `Slot Index In`))
  (if (`self.Validate Slot` `Slot Index In`)
    (`KismetArrayLibrary.Array_Set` (`.TileSlots_4_070D6DA14DE285DA696B848F45A7A9A6` (break `/Game/Blueprints/Structures/LevelGrid/MyTileGridZ` (`|GetArrayItem` (`.ZAxis_3_2D884935497BCE97B635888E43E3AA98` (break `/Game/Blueprints/Structures/LevelGrid/MyTileGridY` (`|GetArrayItem` (`.YAxis_3_B19D8BF7491D421C533931BC366B0A92` (break `/Game/Blueprints/Structures/LevelGrid/MyTileGridX` (`self.Grid`))) _x))) _y))) _z `New Slot In`)
    (return `New Slot In`)))

(fn `Spawn Neighbor Tile`
  (params (`Slot Index In` :type "IntVector Structure") (Direction :type Integer) (`Tile Spawned` :type Boolean))
  (bind _slot_out (`self.Get Slot` `Slot Index In`))
  (if (`.TileSpawned_9_E5F479944C63E28DBE795DA58B6154F7` (break `/Game/Blueprints/Structures/LevelGrid/MyTileSlot` _slot_out))
    (bind _array (`self.Get Tile Connections As Array` (`|GetArrayItem` (break `/Game/Blueprints/Structures/LevelGrid/MyTileSlot` _slot_out))))
    (if (and (!= (`KismetMathLibrary.Conv_ByteToInt` 0) (`KismetMathLibrary.Conv_ByteToInt` (`|GetArrayItem` _array Direction))) (not `Tile Spawned`))
      (`self.Spawn Tile` `Slot Index In`))))

(fn `Spawn Next Tile`
  (bind _best_tile_slots (`self.Best Tile Slots`))
  (bind _tile_count (`self.Tile Count`))
  (bind _best_tile_slots_2 (`self.Best Tile Slots`))
  (set `self.Tile Count` 9999)
  (`KismetArrayLibrary.Array_Clear` (`self.Best Tile Slots`))
  (for _array_element (`self.Next Tile Slots`)
    (bind _slot_out (`self.Get Slot` _array_element))
    (if (and (not (`.TileSpawned_9_E5F479944C63E28DBE795DA58B6154F7` (break `/Game/Blueprints/Structures/LevelGrid/MyTileSlot` _slot_out))) (`self.Validate Slot` _array_element))
      (bind _returnvalue (`KismetArrayLibrary.Array_Length` (break `/Game/Blueprints/Structures/LevelGrid/MyTileSlot` _slot_out)))
      (if (> _returnvalue 1)
        (if (< _returnvalue _tile_count)
          (set `self.Tile Count` _returnvalue)
          (`KismetArrayLibrary.Array_Clear` _best_tile_slots_2)
          (`KismetArrayLibrary.Array_AddUnique` _best_tile_slots_2 _array_element :!label _label)
          (elif (== _returnvalue _tile_count)
            (goto _label)))
        (elif (and (== _returnvalue 1) (not (`.TileSpawned_9_E5F479944C63E28DBE795DA58B6154F7` (break `/Game/Blueprints/Structures/LevelGrid/MyTileSlot` _slot_out))))
          (`self.Spawn Tile` _array_element)))
      (else
        (`KismetArrayLibrary.Array_RemoveItem` (`self.Next Tile Slots`) _array_element))))
  (if (> (`KismetArrayLibrary.Array_Length` _best_tile_slots) 0)
    (set `self.Current Slot` (`KismetArrayLibrary.Array_Random` _best_tile_slots))
    (`self.Spawn Tile` (`self.Current Slot`))
    (set `self.Purge Slots` true)
    (elif (> (`KismetArrayLibrary.Array_Length` (`self.Next Tile Slots`)) 0)
      (`self.Try Spawn Next Tile Again`)
      (else
        (bind _outactors (`GameplayStatics.GetAllActorsOfClass` "/Game/Blueprints/MyTile.MyTile_C"))
        (`KismetSystemLibrary.PrintString` (`KismetStringLibrary.Conv_IntToString` (`KismetArrayLibrary.Array_Length` _outactors)) true true (struct :`R` 0.633333 :`G` 1.0 :`A` 1.0) 60.0)
        (set `self.Generation Complete` true)))))

(fn `Spawn Tile`
  (params (`Slot Index In` :type "IntVector Structure"))
  (locals (`Temp Generated Tile` :type "/Game/Blueprints/MyTile Class Reference") (`Temp Slot` :type "IntVector Structure") (`Temp Connections Array` :type "Array of /Game/Blueprints/ConnectionKeys Enum"))
  (bind _temp_slot (`local.Temp Slot`))
  (bind _tile_position_out (`self.Get Tile Pos` (`local.Temp Slot`)))
  (bind _output_get (set `local.Temp Slot` `Slot Index In`))
  (bind _slot_out (`self.Get Slot` _output_get))
  (if (`.TileSpawned_9_E5F479944C63E28DBE795DA58B6154F7` (break `/Game/Blueprints/Structures/LevelGrid/MyTileSlot` _slot_out))
    (bind _array (`self.Get Tile Connections As Array` (`|GetArrayItem` (break `/Game/Blueprints/Structures/LevelGrid/MyTileSlot` _slot_out))))
    (set `local.Temp Connections Array` _array)
    (for (_array_element _array_index) (`self.Get Directional Vectors`) :!label _label
      (bind _int_vector_out (`self.Add Int Vector` _array_element _temp_slot))
      (bind _slot_out_2 (`self.Get Slot` _int_vector_out))
      (if (and (!= (`KismetMathLibrary.Conv_ByteToInt` 0) (`KismetMathLibrary.Conv_ByteToInt` (`|GetArrayItem` (`local.Temp Connections Array`) _array_index))) (not (`.TileSpawned_9_E5F479944C63E28DBE795DA58B6154F7` (break `/Game/Blueprints/Structures/LevelGrid/MyTileSlot` _slot_out_2))))
        (`KismetArrayLibrary.Array_AddUnique` (`self.Next Tile Slots`) _int_vector_out)))
    (`KismetArrayLibrary.Array_AddUnique` (`self.Slots To Purge`) _temp_slot)
    (`KismetArrayLibrary.Array_RemoveItem` (`self.Next Tile Slots`) (`self.Current Slot`))
    (else
      (bind _output_get_2 (set `local.Temp Generated Tile` (`|GetArrayItem` (break `/Game/Blueprints/Structures/LevelGrid/MyTileSlot` _slot_out) (`KismetMathLibrary.RandomInteger` (`KismetArrayLibrary.Array_Length` (break `/Game/Blueprints/Structures/LevelGrid/MyTileSlot` _slot_out))))))
      (if (`KismetSystemLibrary.IsValidClass` _output_get_2)
        (`|SpawnActorFromClass` _output_get_2 (`KismetMathLibrary.MakeTransform` _tile_position_out (struct) (`KismetMathLibrary.Conv_DoubleToVector` (`self.Tiles Scale`))) "Undefined" "MultiplyWithRoot" null null)
        (if (`self.Debug Tile Bounds`)
          (`KismetSystemLibrary.DrawDebugBox` _tile_position_out (`KismetMathLibrary.Conv_DoubleToVector` (/ (`self.Tile Spacing`) 2.0)) (struct :`R` 1.0 :`B` 0.016666 :`A` 1.0) (struct) 300.0 5.0))
        (`self.Set Slot` (`local.Temp Slot`) (make `/Game/Blueprints/Structures/LevelGrid/MyTileSlot` (`|MakeArray` _output_get_2) true))
        (bind _array_2 (`self.Get Tile Connections As Array` _output_get_2))
        (set `local.Temp Connections Array` _array_2)
        (goto _label)))))

(fn `UserConstructionScript`)

(fn `Validate Slot`
  (params (`Slot Index In` :type "IntVector Structure (by ref)"))
  (returns (`Slot is Valid` :type Boolean))
  (bind (_x _y _z) (break `IntVector` `Slot Index In`))
  (bind (_grid_size_out_x _grid_size_out_y _grid_size_out_z) (break `IntVector` (`self.Get Grid Size`)))
  (return (not (`KismetArrayLibrary.Array_Contains` (`|MakeArray` (>= _x 0) (< _x _grid_size_out_x) (>= _y 0) (< _y _grid_size_out_y) (>= _z 0) (< _z _grid_size_out_z))))))