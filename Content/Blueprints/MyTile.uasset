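; MyTile is a tile actor that carries a mesh, a yaw rotation and connection keys for its six axis directions.
; Its construction script applies the mesh and rotation, then either labels the connections for debugging or hides the debug text and its children.
; Labels come from index-matched helper lists of keys, text components and direction vectors.
; A separate helper can spawn connection text components but is not called here.
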(fn `Add Connection Debug Text`
  (params (Direction :type "Vector Structure (by ref)") (`Connection Key` :type String))
  (bind _returnvalue (`AddComponent|NODE_AddTextRenderComponent-0` :`RelativeTransform` (`KismetMathLibrary.MakeTransform` Direction (`KismetMathLibrary.FindLookAtRotation` (`self.K2_GetActorLocation`) Direction))))
  (`TextRenderComponent.K2_SetText` _returnvalue (`KismetTextLibrary.Conv_StringToText` `Connection Key`)))

(fn `UserConstructionScript`
  (bind (_forward_x _backward_x _right_y _left_y _up_z _down_z) (break `/Game/Blueprints/Structures/Connections/TileConnections` (`self.Tile Connections`)))
  (`StaticMeshComponent.SetStaticMesh` (`self.M_TileMesh`) (`self.Tile Mesh`))
  (`SceneComponent.K2_SetRelativeRotation` (`self.M_TileMesh`) (`KismetMathLibrary.MakeRotator` 0.0 0.0 (`self.Rotation`)) false false)
  (if (`self.Debug Connections`)
    (for (_array_element _array_index) (`|MakeArray` _forward_x _backward_x _right_y _left_y _up_z _down_z)
      (bind _output (`|GetArrayItem` (`|MakeArray` (`self.Right`) (`self.Left`) (`self.Forward`) (`self.Backward`) (`self.Up`) (`self.Down`)) _array_index))
      (`TextRenderComponent.K2_SetText` _output (`KismetTextLibrary.Conv_StringToText` (`|GetEnumeratorNameAsString` _array_element)))
      (`SceneComponent.K2_SetRelativeLocation` _output (* (`|GetArrayItem` (`|MakeArray` (`KismetMathLibrary.Vector_Forward`) (`KismetMathLibrary.Vector_Backward`) (`KismetMathLibrary.Vector_Right`) (`KismetMathLibrary.Vector_Left`) (`KismetMathLibrary.Vector_Up`) (`KismetMathLibrary.Vector_Down`)) _array_index) (`self.Debug Text Distance`)) false false))
    (else
      (`SceneComponent.SetVisibility` (`self.Debug Text`) false true))))